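; AI controller that drives a patrolling BP_Enemy through the BT_AIPatrol behavior tree.
; On BeginPlay it starts the tree, caches the controlled enemy and copies its patrol path's looping setting to the blackboard.
; When AI perception senses a ThirdPersonCharacter, it flags CanSeePlayer, sets Direction to forward one and copies the path's wait time.
; Losing sight is not handled here, so this graph never clears CanSeePlayer.
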(event OnTargetPerceptionUpdated(AIPerception)
  (params (Actor :type Actor%20Object%20Reference) (Stimulus :type AI%20Stimulus%20Structure))
  (bind _returnvalue (AI|GetBlackboard 0))
  (Utilities|Casting|CastToThirdPersonCharacter Actor)
  (if (.bSuccessfullySensed (Utilities|Struct|BreakAIStimulus Stimulus))
    (AI|Components|Blackboard|SetValueasBool (AI|GetBlackboard 0) (Utilities|Name|MakeLiteralName "CanSeePlayer") true)
    (Class|BlackboardComponent|SetValueasInt _returnvalue (Utilities|Name|MakeLiteralName "Direction") 1)
    (AI|Components|Blackboard|SetValueasFloat _returnvalue (Utilities|Name|MakeLiteralName "WaitTime") (Variables|/Game/Blueprints/BP_PatrolPath.BP_PatrolPath_C|GetWaitTime (Variables|/Game/Blueprints/BP_Enemy.BP_Enemy_C|GetPatrolPath (Variables|Default|GetCustomPawn))))))

(event EventBeginPlay
  (AI|RunBehaviorTree "/Game/Blueprints/BT_AIPatrol.BT_AIPatrol")
  (bind _asbp_enemy (Utilities|Casting|CastToBP_Enemy (Pawn|GetControlledPawn)))
  (bind _output_get (Variables|Default|SetCustomPawn _asbp_enemy))
  (AI|Components|Blackboard|SetValueasBool (AI|GetBlackboard 0) (Utilities|Name|MakeLiteralName "PathLooping") (Variables|/Game/Blueprints/BP_PatrolPath.BP_PatrolPath_C|GetIsLooping (Variables|/Game/Blueprints/BP_Enemy.BP_Enemy_C|GetPatrolPath _output_get))))

(event EventTick
  (params (DeltaSeconds :type Float%20%28single-precision%29)))

(fn ConstructionScript)